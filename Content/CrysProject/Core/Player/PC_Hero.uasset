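; PC_Hero is the hero player controller Blueprint, which shows a lock-on marker on the current target for the local player.
; It listens for target point changes from the TargetingSystemComponent.
; A valid point spawns the NS_LockOn Niagara system attached to that point's component and socket, or re-attaches the existing one.
; An invalid point destroys the marker.
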(event OnTargetPointChangedDelegate(TargetingSystemComponent)
  (params (OldTargetPoint :type Crim%20Target%20Point%20Structure%20%28by%20ref%29) (NewTargetPoint :type Crim%20Target%20Point%20Structure%20%28by%20ref%29))
  (bind (_weakscenecomponent _socketname) (Utilities|Struct|BreakCrimTargetPoint NewTargetPoint))
  (if (Pawn|IsLocalPlayerController)
    (if (Class|CrimTargetingSystemBlueprintFunctionLibrary|IsTargetPointValid NewTargetPoint)
      (bind _lockonsystem (Variables|Default|GetLockOnSystem)
        (:then
          (Transformation|AttachComponentToComponent _lockonsystem _weakscenecomponent _socketname "KeepRelative" "KeepRelative" "KeepRelative" false))
        (:else
          (bind _returnvalue (Niagara|SpawnSystemAttached "/Game/CrysProject/NiagaraSystem/NS_LockOn.NS_LockOn" _weakscenecomponent _socketname "0, 0, 0" "0, 0, 0" "KeepRelativeOffset" false))
          (Variables|Default|SetLockOnSystem _returnvalue)))
      (else
        (bind _lockonsystem_2 (Variables|Default|GetLockOnSystem)
          (:then
            (Components|DestroyComponent _lockonsystem_2))
          (:else))))))

(event EventBeginPlay)

(event EventTick
  (params (DeltaSeconds :type Float%20%28single-precision%29)))

(fn ConstructionScript)